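; BP_SubInvoker is an actor that alternates between two numbered streaming levels through a stream level manager.
; Each ToggleGivenLevelsStreamState call increments a counter, whose parity picks which "StreamLevel" plus target index name to load and which to remove.
; It passes itself as notification receiver, and its LevelSwitchFinished event sets custom primitive data on its Sphere, presumably as a visual cue.
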(event `self.LevelSwitchFinished`
  (params (bFinishAll :type Boolean))
  (`PrimitiveComponent.SetCustomPrimitiveDataFloat` (`self.Sphere`) 0 1.0))

(fn `ToggleGivenLevelsStreamState`
  (bind _set (`|MakeSet` "None" :!type "Name"))
  (bind _returnvalue (== (mod (`self.ToggleCounter`) 2) 1))
  (bind _set_2 (`|MakeSet` (`KismetStringLibrary.Conv_StringToName` (`KismetStringLibrary.Concat_StrStr` "StreamLevel" (`KismetStringLibrary.Conv_IntToString` (`self.TargetLevelIndex2`))))))
  (bind _set_3 (`|MakeSet` (`KismetStringLibrary.Conv_StringToName` (`KismetStringLibrary.Concat_StrStr` "StreamLevel" (`KismetStringLibrary.Conv_IntToString` (`self.TargetLevelIndex1`))))))
  (`/Engine/EditorBlueprintResources/StandardMacros.IncrementInt` (`self.ToggleCounter`)
    (:`  `
      (`MyStreamLevelManager.SwitchStreamLevels` (subsystem `MyStreamLevelManager`) _set _set (select `bool` _returnvalue :`false` _set_2 :`true` _set_3) (select `bool` _returnvalue :`false` _set_3 :`true` _set_2) self))))

(fn `UserConstructionScript`)