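; Debug actor that exercises the stream level manager's level switching and completion notifications.
; Debug key O requests unloading all current stream levels, waits briefly, binds an all-finished callback, then toggles every BP_SubInvoker's levels.
; Debug key P prints the current stream levels, and notification handlers print completion messages.
; Unconnected graphs hold alternative tests: preset data assets with custom overrides, single-function switching, separate load/unload calls and step-counted delegate binding.
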(event Custom|OnLoadUnloadFInished
  (params (bIsLoadCommand :type Boolean))
  ;[1 1 1] 使用多播委托
  (Development|PrintString (Utilities|String|SelectString "Load Commands Finished" "Unload Commands Finished" bIsLoadCommand))
  (bind _result (Math|Integer|DecrementInt (Variables|Default|GetStepCount))
    (:%20%20
      (if (== _result 0)
        (EventDispatchers|UnbindEventfromOnTrySwitchLevelFinished (Subsystems|GetMyStreamLevelManager) (delegate Custom|OnLoadUnloadFInished))
        (Development|PrintString "All Command Finished Unbind Delegate")))))

(event Custom|AllFinished
  ;[1 1 1] 调用场景内5个触发器的切换行为
  (Development|PrintString "All Command Finished" true true "(R=0.000000,G=0.660000,B=1.000000,A=1.000000)" 2e+01))

(event EventBeginPlay
  (bind _returnvalue (Actor|GetActorOfClass "/Game/BP_InterfaceNotifyReceiver.BP_InterfaceNotifyReceiver_C"))
  (Variables|Default|SetReceiver _returnvalue))

(event Collision|EventActorBeginOverlap
  (params (OtherActor :type Actor%20Object%20Reference)))

(event EventTick
  (params (DeltaSeconds :type Float%20%28single-precision%29)))

(event EventTrySwitchFinished
  (params (bIsLoadCommand :type Boolean))
  (Development|PrintString "Load Commands Finished,Told By Interface"))

(event Input|KeyboardEvents|DebugKeyO
  (params (Key :type Key%20Structure :default "None") (ActionValue :type Input%20Action%20Value%20Structure))
  (bind _returnvalue (Subsystems|GetMyStreamLevelManager))
  (:Pressed
    ;[1 1 1] 卸载所有关卡
    (Class|MyStreamLevelManager|TryUnloadSomeLevels _returnvalue (Class|MyStreamLevelManager|GetCurrentStreamLevels _returnvalue) self)
    (Utilities|FlowControl|Delay 5.0)
    ;[1 1 1] 调用场景内5个触发器的切换行为
    (EventDispatchers|BindEventtoSwitchAllStreamLevelFinished (Subsystems|GetMyStreamLevelManager) (delegate Custom|AllFinished))
    (bind _outactors (Actor|GetAllActorsOfClass "/Game/BP_SubInvoker.BP_SubInvoker_C"))
    (for _array_element _outactors
      (Default|ToggleGivenLevelsStreamState _array_element))))

(event Input|KeyboardEvents|DebugKeyP
  (params (Key :type Key%20Structure :default "None") (ActionValue :type Input%20Action%20Value%20Structure))
  (:Pressed
    ;[1 1 1] 打印当前已加载的关卡名称
    (bind _result (Utilities|Set|ToArray (Class|MyStreamLevelManager|GetCurrentStreamLevels (Subsystems|GetMyStreamLevelManager))))
    (for _array_element _result
      (Development|PrintString (Utilities|String|ToString(Name) _array_element)))))

(fn ConstructionScript)